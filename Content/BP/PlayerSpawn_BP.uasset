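; PlayerSpawn_BP is a spawn zone that tracks whether its assigned player is standing inside, apparently for a fencing mode.
; ActiveSpawn and DeactiveSpawn toggle IsActive and show or hide the Cube marker, which starts hidden.
; While active, Box overlap begin and end set PlayerIsReady for CurrentPlayer only.
; Both paths then cast the game mode to FencingGameMode_BP, with no further action after the cast.
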(event OnComponentBeginOverlap(Box)
  (params (OverlappedComponent :type Primitive%20Component%20Object%20Reference) (OtherActor :type Actor%20Object%20Reference) (OtherComp :type Primitive%20Component%20Object%20Reference) (OtherBodyIndex :type Integer) (bFromSweep :type Boolean) (SweepResult :type Hit%20Result%20Structure%20%28by%20ref%29))
  (if (Variables|Default|GetIsActive)
    (if (== OtherActor (Variables|Default|GetCurrentPlayer))
      (Variables|Default|SetPlayerIsReady true)
      (Utilities|Casting|CastToFencingGameMode_BP (Game|GetGameMode)))))

(event OnComponentEndOverlap(Box)
  (params (OverlappedComponent :type Primitive%20Component%20Object%20Reference) (OtherActor :type Actor%20Object%20Reference) (OtherComp :type Primitive%20Component%20Object%20Reference) (OtherBodyIndex :type Integer))
  (if (Variables|Default|GetIsActive)
    (if (== (Variables|Default|GetCurrentPlayer) OtherActor)
      (Variables|Default|SetPlayerIsReady false)
      (Utilities|Casting|CastToFencingGameMode_BP (Game|GetGameMode)))))

(event Custom|ActiveSpawn
  (Variables|Default|SetIsActive true)
  (Development|SetHiddeninGame (Variables|Default|GetCube) false false))

(event Custom|DeactiveSpawn
  (Variables|Default|SetIsActive false)
  (Development|SetHiddeninGame (Variables|Default|GetCube) true false))

(event EventBeginPlay
  (Development|SetHiddeninGame (Variables|Default|GetCube) true false))

(event Collision|EventActorBeginOverlap
  (params (OtherActor :type Actor%20Object%20Reference)))

(event EventTick
  (params (DeltaSeconds :type Float%20%28single-precision%29)))

(fn ConstructionScript)