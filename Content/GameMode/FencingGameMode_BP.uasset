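; Game mode for a two-player fencing match that tracks scores and gates play on player readiness.
; ManagePoint awards more for head hits than other hits, then calls ReplacePlayer, which locks play but only prints a debug string.
; CheckPlayerReady unlocks play and calls StartMatch when every spawned player's sword is ready.
; StartMatch and respawning are stubs, and BeginPlay's spawn lookup is never stored in PlayerSpawns.
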(event Custom|ReplacePlayer
  (Variables|Default|SetCantPlay true)
  (Development|PrintString "Hello")
  (for _array_element (Variables|Default|GetPlayerSpawns)
    _))

(event Custom|StartMatch
  (for _array_element (Variables|Default|GetPlayerSpawns)
    _))

(event Custom|ManagePoint
  (params (PlayerIndex :type Integer) (HitLocation :type String))
  (if (Utilities|Enum|Equal(Enum) HitLocation "Head")
    (Variables|Default|SetTempScore 3)
    (else
      (Variables|Default|SetTempScore 1)))
  (if (== PlayerIndex 0)
    (Variables|Default|SetScorePlayer1 (+ (Variables|Default|GetScorePlayer1) (Variables|Default|GetTempScore)))
    (else
      (Variables|Default|SetScorePlayer2 (+ (Variables|Default|GetScorePlayer2) (Variables|Default|GetTempScore)))))
  (CallFunction|ReplacePlayer))

(event Custom|CheckPlayerReady
  (Variables|Default|SetIsPlayerAreReady true)
  (for _array_element (Variables|Default|GetPlayerSpawns)
    (if (not true)
      (Variables|Default|SetIsPlayerAreReady false)))
  (if (Variables|Default|GetIsPlayerAreReady)
    (Variables|Default|SetCantPlay false)
    (for _array_element_2 (Variables|Default|GetPlayerSpawns)
      (if (not (Variables|/Game/BP/VrPawn_BP.VrPawn_BP_C|GetSwordIsReady (Variables|/Game/BP/PlayerSpawn_BP.PlayerSpawn_BP_C|GetCurrentPlayer _array_element_2)))
        (Variables|Default|SetIsPlayerAreReady false)))
    (if (Variables|Default|GetIsPlayerAreReady)
      (Variables|Default|SetCantPlay false)
      (CallFunction|StartMatch)
      (else
        (Variables|Default|SetCantPlay true)))))

(event EventBeginPlay
  (Actor|GetAllActorsOfClass "/Game/BP/PlayerSpawn_BP.PlayerSpawn_BP_C"))

(event EventTick
  (params (DeltaSeconds :type Float%20%28single-precision%29)))

(fn ConstructionScript)